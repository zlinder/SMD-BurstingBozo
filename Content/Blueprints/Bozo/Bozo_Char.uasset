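; Bozo_Char is an enemy character that animates out of what appears to be a crate, then pursues the player and can be shot for points.
; On BeginPlay a timeline offsets the capsule along X and Z, then AIMoveTo targets the player's camera manager.
; A projectile overlapping its Box calls WasHit, then once only awards score, hides the mesh, spawns a particle effect and destroys the actor after a short delay.
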(event `self.Box.OnComponentBeginOverlap`
  (params (OverlappedComponent :type "PrimitiveComponent Object Reference") (OtherActor :type "Actor Object Reference") (OtherComp :type "PrimitiveComponent Object Reference") (OtherBodyIndex :type Integer) (bFromSweep :type Boolean) (SweepResult :type "HitResult Structure (by ref)"))
  (cast `/Game/Blueprints/Player/BP_Projectile` OtherActor)
  (`/Game/Blueprints/Interface/BPI_Enemy.WasHit`)
  (`/Engine/EditorBlueprintResources/StandardMacros.DoOnce` false
    (:`Completed`
      (message `/Game/Blueprints/Interface/BPI_Player.AddToScore` (`GameplayStatics.GetPlayerPawn` 0) 50)
      (`SceneComponent.SetVisibility` (`self.Mesh`) false false)
      (`GameplayStatics.SpawnEmitterAtLocation` "/Game/VRGunToolkit/Particles/Weapons/P_AssaultRifle_MF.P_AssaultRifle_MF" (`self.K2_GetActorLocation`))
      (`KismetSystemLibrary.Delay` 0.75)
      (`self.K2_DestroyActor`))))

(event `self.ReceiveBeginPlay`
  (bind (_direction _crateexitz _crateexitx) (`Timeline|Timeline_0`)
    (:`Update`
      (`SceneComponent.K2_AddRelativeLocation` (`self.CapsuleComponent`) (`KismetMathLibrary.MakeVector` _crateexitx 0.0 _crateexitz) false false))
    (:`Finished`
      (`|AIMoveTo` self (0.0 0.0 0.0) (`GameplayStatics.GetPlayerCameraManager` 0)))))

(fn `UserConstructionScript`)