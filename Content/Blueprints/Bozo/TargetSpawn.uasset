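; TargetSpawn is a spawner actor that keeps one AI pawn of a configurable class alive at its location.
; It spawns the pawn on BeginPlay via SpawnAIFromClass and stores the reference in SpawnedEnem.
; Tick polls that reference and, once it is invalid, waits SpawnTime through a Delay before calling Respawn to spawn a replacement.
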(event `Respawn`
  (bind _returnvalue (`AIBlueprintHelperLibrary.SpawnAIFromClass` (`self.Class to Spawn`) null (`self.K2_GetActorLocation`) :!label _label))
  (set `self.SpawnedEnem` _returnvalue))

(event `self.ReceiveBeginPlay`
  (goto _label))

(event `self.ReceiveTick`
  (params (DeltaSeconds :type "Float (single-precision)"))
  (if (not (`KismetSystemLibrary.IsValid` (`self.SpawnedEnem`)))
    (`KismetSystemLibrary.Delay` (`self.SpawnTime`))
    (`self.Respawn`)))

(fn `UserConstructionScript`)