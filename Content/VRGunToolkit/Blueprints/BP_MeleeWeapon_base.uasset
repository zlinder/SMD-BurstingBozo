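; BP_MeleeWeapon_base is a melee weapon Blueprint in VRGunToolkit that deals impact-based damage and can stick into surfaces.
; On Hit, it maps impulse magnitude through the PhysicalHitSound impact thresholds to damage between zero and MaxDamage.
; When Pierce is enabled, a sufficiently hard PiercingVolume hit on a non-simulating component attaches the SMKnive component to it, keeping its world transform.
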(event `self.ReceiveHit`
  (params (MyComp :type "PrimitiveComponent Object Reference") (Other :type "Actor Object Reference") (OtherComp :type "PrimitiveComponent Object Reference") (bSelfMoved :type Boolean) (HitLocation :type "Vector Structure") (HitNormal :type "Vector Structure") (NormalImpulse :type "Vector Structure") (Hit :type "HitResult Structure (by ref)"))
  (bind _physicalhitsound (`self.PhysicalHitSound`))
  ;[1 1 1] Damage Based on impact velocity
  (`GameplayStatics.ApplyDamage` Other (`KismetMathLibrary.MapRangeClamped` (`KismetMathLibrary.VSize` NormalImpulse) (`/Game/VRGunToolkit/Blueprints/Physics/PhysicalHitSound.ThreshholdImpactMin` _physicalhitsound) (`/Game/VRGunToolkit/Blueprints/Physics/PhysicalHitSound.ThreshholdImpactMax` _physicalhitsound) 0.0 (`self.MaxDamage`))))

(event `self.PiercingVolume.OnComponentHit`
  (params (HitComponent :type "PrimitiveComponent Object Reference") (OtherActor :type "Actor Object Reference") (OtherComp :type "PrimitiveComponent Object Reference") (NormalImpulse :type "Vector Structure") (Hit :type "HitResult Structure (by ref)"))
  ;[1 1 1] Piercing (stuck knife)
  (if (and (not (`SceneComponent.IsSimulatingPhysics` OtherComp "None")) (> (`KismetMathLibrary.VSize` NormalImpulse) 100.0) (`self.Pierce`))
    (`SceneComponent.K2_AttachToComponent` (`self.SM_Knive`) OtherComp "None" "KeepWorld" "KeepWorld" "KeepWorld" true)))

(fn `UserConstructionScript`)