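; Component in the VR gun toolkit that plays impact sounds when its owning physical actor hits something.
; After a one-second BeginPlay delay to skip spawn drops, it binds to the owner's hit event.
; ValidHit filters hits by cooldown and impulse threshold, plus either enough transform change or a brief gap since the last rejected hit.
; Normalized impulse strength scales volume and pitch of the attenuated, concurrency-limited sound at the hit location.
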(event `self.ReceiveBeginPlay`
  ;[0.6208 0.765 1] Small delay to avoid begin play drop sounds
  (`KismetSystemLibrary.Delay` 1.0)
  (add `Actor.OnActorHit` (`self.GetOwner`) (delegate `OwnerActorHit`)))

(event `OwnerActorHit`
  (params (SelfActor :type "Actor Object Reference") (OtherActor :type "Actor Object Reference") (NormalImpulse :type "Vector Structure") (Hit :type "HitResult Structure (by ref)"))
  ;[1 0.843 0.5412] When the actor is hit, we see if there's enough strenght to trigger a hit sound, if yes we play sound at the hit location
  (bind _valid (`self.ValidHit` NormalImpulse))
  (if _valid
    (`GameplayStatics.PlaySoundAtLocation` (`self.HitSound`) Hit_Location (struct) (`KismetMathLibrary.MapRangeClamped` (`self.HitStrength`) 0.0 1.0 (`self.VolumeMin`) (`self.VolumeMax`)) (`KismetMathLibrary.MapRangeClamped` (`self.HitStrength`) 0.0 1.0 0.85 1.15) 0.0 "/Game/VRGunToolkit/Sounds/Shells/DropSoundAttenuation.DropSoundAttenuation" "/Game/VRGunToolkit/Sounds/Shells/DropSoundConcurrency.DropSoundConcurrency")
    (set `self.LastTriggerGameTime` (`KismetSystemLibrary.GetGameTimeInSeconds`))
    (set `self.LastTriggerTransform` (`Actor.GetTransform` (`self.GetOwner`)))))

(fn `ValidHit`
  (params (NewParam :type "Vector Structure"))
  (returns (Valid :type Boolean))
  (set `self.HitStrength` (`KismetMathLibrary.VSize` NewParam))
  (if (and (>= (- (`KismetSystemLibrary.GetGameTimeInSeconds`) (`self.LastTriggerGameTime`)) (`self.RetriggerCooldown`)) (>= (`self.HitStrength`) (`self.ThreshholdImpactMin`)) (or (not (`KismetMathLibrary.NearlyEqual_TransformTransform` (`self.LastTriggerTransform`) (`Actor.GetTransform` (`self.GetOwner`)) (`self.TriggerLocationDeltaThreshold`) (`self.TriggerRotationDeltaThreshold`))) (>= (- (`KismetSystemLibrary.GetGameTimeInSeconds`) (`self.LastInvalidHitGameTime`)) 0.01)))
    (set `self.HitStrength` (`KismetMathLibrary.MapRangeClamped` (`self.HitStrength`) (`self.ThreshholdImpactMin`) (`self.ThreshholdImpactMax`) 0.0 1.0))
    (return true)
    (else
      (set `self.LastInvalidHitGameTime` (`KismetSystemLibrary.GetGameTimeInSeconds`))
      (return false))))